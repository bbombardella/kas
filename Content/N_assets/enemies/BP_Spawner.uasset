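; BP_Spawner is an enemy spawner that periodically spawns Keuf1 actors around player 0's pawn.
; A looping timer started on BeginPlay calls SpawnMob, which offsets the player's location horizontally using SpawnRadius.
; X and Y use separate random angles, so spawns scatter within a square rather than on a circle.
; A random three-way switch currently routes every case to the same Keuf1 spawn.
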(event EventBeginPlay
  (Utilities|Time|SetTimerbyFunctionName 0 "SpawnMob" 5.0 true))

(fn ConstructionScript)

(fn SpawnMob
  (bind _returnvalue (Math|Random|RandomFloatinRange 0.0 3.6e+02))
  (bind _spawnradius (Variables|Default|GetSpawnRadius))
  (bind _returnvalue_2 (Math|Trig|DegreesToRadians _returnvalue))
  (bind _output_get (Variables|Default|SetPlayerLocation (Transformation|GetActorLocation (Game|Player|GetPlayerPawn 0))))
  (switch int (Math|Conversions|ToInteger(Byte) (Class|KismetMathLibrary|RandomInteger64inRange 0 2))
    (:0
      _)
    (:1
      _)
    (:2
      _))
  (Game|SpawnActorfromClass "/Game/N_assets/enemies/keuf_1/Keuf1.Keuf1_C" (Math|Conversions|ToTransform(Vector) (+ (Math|Vector|MakeVector (* (Math|Trig|Cos(Radians) _returnvalue_2) _spawnradius) (* (Math|Trig|Sin(Radians) _returnvalue_2) _spawnradius) 0.0) _output_get)) "Undefined" "MultiplyWithRoot" 0 0))