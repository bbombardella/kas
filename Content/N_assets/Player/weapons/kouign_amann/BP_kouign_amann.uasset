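; BP_kouign_amann is a player weapon actor that circles around its owner.
; Each Tick advances an angle by Speed times delta time, then sets the actor's location from its cosine and sine scaled by Radius.
; The orbit centers on the owner's current X and Y, while Z does not follow the owner.
; The graph holds no overlap or damage logic.
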(event EventBeginPlay)

(event Collision|EventActorBeginOverlap
  (params (OtherActor :type Actor%20Object%20Reference)))

(event EventTick
  (params (DeltaSeconds :type Float%20%28single-precision%29))
  (bind _returnvalue (Components|GetOwner))
  (bind _radius (Variables|Default|Getradius))
  (bind _returnvalue_2 (Transformation|GetActorLocation _returnvalue))
  (bind _output_get (Variables|Default|Setangle (+ (Variables|Default|Getangle) (* DeltaSeconds (Variables|Default|Getspeed)))))
  (Transformation|SetActorLocation (Math|Vector|MakeVector (+ (* (Math|Trig|Cos(Radians) (Math|Trig|DegreesToRadians _output_get)) _radius) (.x _returnvalue_2)) (+ (.y _returnvalue_2) (* _radius (Math|Trig|Sin(Radians) (Math|Trig|DegreesToRadians _output_get)))) 0.0) false false))

(fn ConstructionScript)