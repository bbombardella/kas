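; BP_triskèle is a player weapon projectile that flies in a straight line and destroys Characters it overlaps.
; On BeginPlay it takes its direction from the player pawn toward its own location and starts a short timer to destroy itself.
; Tick moves it with a swept, delta-time-scaled offset.
; The capsule overlap destroys any Character outright, with no damage step or player check, and the projectile keeps flying.
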(event OnComponentBeginOverlap(Capsule)
  (params (OverlappedComponent :type Primitive%20Component%20Object%20Reference) (OtherActor :type Actor%20Object%20Reference) (OtherComp :type Primitive%20Component%20Object%20Reference) (OtherBodyIndex :type Integer) (bFromSweep :type Boolean) (SweepResult :type Hit%20Result%20Structure%20%28by%20ref%29))
  (bind _ascharacter (Utilities|Casting|CastToCharacter OtherActor))
  (Actor|DestroyActor _ascharacter))

(event EventTick
  (params (DeltaSeconds :type Float%20%28single-precision%29))
  (Transformation|AddActorWorldOffset (* (Variables|Default|GetDirection) (Utilities|Time|GetWorldDeltaSeconds) (Variables|Default|Getspeed)) true))

(event EventBeginPlay
  (Variables|Default|SetDirection (Math|Vector|Normalize (- (Transformation|GetActorLocation) (Transformation|GetActorLocation (Game|Player|GetPlayerPawn 0)))))
  (Utilities|Time|SetTimerbyFunctionName 0 "destroySelf" 1.5))

(fn ConstructionScript)

(fn DestroySelf
  (Actor|DestroyActor))