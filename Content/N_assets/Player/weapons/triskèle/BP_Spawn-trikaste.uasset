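; Spawner Blueprint that creates a BP_triskèle actor near the player pawn each time the Space Bar is released.
; The spawn location offsets the pawn's position horizontally using cosine and sine scaled by SpawnRadius, at the pawn's height.
; X and Y each draw their own random angle, so spawns scatter within a square around the player instead of lying on a circle.
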(event Input|KeyboardEvents|SpaceBar
  (params (Key :type Key%20Structure :default "None"))
  (bind _returnvalue (Math|Random|RandomFloatinRange 0.0 3.6e+02))
  (bind _spawnradius (Variables|Default|GetspawnRadius))
  (bind _returnvalue_2 (Math|Trig|DegreesToRadians _returnvalue))
  (:Released
    (Game|SpawnActorfromClass "/Game/N_assets/Player/weapons/triskèle/BP_triskèle.BP_triskèle_C" (Math|Conversions|ToTransform(Vector) (+ (Math|Vector|MakeVector (* (Math|Trig|Cos(Radians) _returnvalue_2) _spawnradius) (* (Math|Trig|Sin(Radians) _returnvalue_2) _spawnradius) 0.0) (Transformation|GetActorLocation (Game|Player|GetPlayerPawn 0)))) "Undefined" "MultiplyWithRoot" 0 0)))

(fn ConstructionScript)