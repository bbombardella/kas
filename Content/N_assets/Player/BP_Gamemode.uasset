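; BP_Gamemode is a player game mode Blueprint that tracks HP and reloads or switches level when it runs out.
; BeginPlay sets HP to full and adds a Health widget to the viewport.
; Tick prints the death check every frame and opens the Kas_mt_sm level once HP reaches zero.
; An unconnected node to destroy the player controller and pawn never runs.
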(event EventBeginPlay
  (Variables|Default|SetHP 1e+02)
  (bind _returnvalue (UserInterface|CreateWidget "/Game/N_assets/ui/Health.Health_C"))
  (UserInterface|Viewport|AddtoViewport _returnvalue 0))

(event EventTick
  (params (DeltaSeconds :type Float%20%28single-precision%29))
  (bind _hp (Variables|Default|GetHP))
  (bind _returnvalue (<= _hp 0.0))
  (Development|PrintString (Utilities|String|ToString(Boolean) _returnvalue) true true "(R=0.000000,G=0.660000,B=1.000000,A=1.000000)" 0.1)
  (if _returnvalue
    (Game|OpenLevel(byObjectReference) "/Game/kas_mt_sm.kas_mt_sm")))

(fn ConstructionScript)